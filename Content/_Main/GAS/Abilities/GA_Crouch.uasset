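; GA_Crouch is a Gameplay Ability that makes the owning MET character crouch while the input is held.
; On activation it crouches the character and waits for input release, which ends the ability; an invalid character ends it immediately.
; Ending the ability uncrouches the character.
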(event Ability|EventActivateAbility
  (bind _output_get (Variables|Default|SetCharacter (Class|METGameplayAbility|GetMetCharacterfromActorInfo)))
  (Utilities|IsValid _output_get
    (:Is%20Valid
      (Character|Crouch (Variables|Default|GetCharacter))
      (Ability|Tasks|WaitInputRelease false
        (:OnRelease
          (Ability|EndAbility))))
    (:Is%20Not%20Valid
      (Ability|EndAbility))))

(event Ability|EventOnEndAbility
  (params (bWasCancelled :type Boolean))
  (bind _character (Variables|Default|GetCharacter)
    (:then
      (Character|UnCrouch _character))
    (:else)))